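; Tank pawn Blueprint that hooks player input to the tank's aiming, movement and camera components.
; On BeginPlay it hands the barrel and turret to the Aiming component and both tracks to TankMovement.
; Axes rotate the azimuth gimbal and spring arm for camera orbit, and Fire triggers the Aiming component.
; Driving works either through direct per-track throttle or through forward and turn intents sent to TankMovement.
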(event `self.ReceiveBeginPlay`
  (`AimingComponent.InitializeAiming` (`self.Aiming`) (`self.Barrel`) (`self.Turret`))
  (`TankMovementComponent.Initialise` (`self.TankMovement`) (`self.LeftTrack`) (`self.RightTrack`)))

(event `InputAxis|Azimuth_Axis`
  (params (AxisValue :type "Float (single-precision)"))
  ;[1 1 1] Camera Parameters
  (`SceneComponent.K2_AddLocalRotation` (`self.Azimuth Gimbal`) (`KismetMathLibrary.MakeRotator` 0.0 0.0 AxisValue) false false))

(event `InputAxis|Left Track Throttle`
  (params (AxisValue :type "Float (single-precision)"))
  ;[1 1 1] Movement Input Binding
  (`TankTrack.SetThrottle` (`self.LeftTrack`) AxisValue))

(event `InputAction|Fire`
  (params (Key :type "Key Structure"))
  ;[1 1 1] Firing Input Binding
  (:`Pressed`
    (`AimingComponent.Fire` (`self.Aiming`))))

(event `InputAxis|Right Track Throttle`
  (params (AxisValue :type "Float (single-precision)"))
  ;[1 1 1] Movement Input Binding
  (`TankTrack.SetThrottle` (`self.RightTrack`) AxisValue))

(event `InputAxis|Altitude_Axis`
  (params (AxisValue :type "Float (single-precision)"))
  ;[1 1 1] Camera Parameters
  (`SceneComponent.K2_AddLocalRotation` (`self.SpringArm`) (`KismetMathLibrary.MakeRotator` 0.0 AxisValue) false false))

(event `InputAxis|MoveForward`
  (params (AxisValue :type "Float (single-precision)"))
  ;[1 1 1] Movement Input Binding
  (`TankMovementComponent.IntendMoveForward` (`self.TankMovement`) AxisValue))

(event `InputAxis|MoveLeft`
  (params (AxisValue :type "Float (single-precision)"))
  ;[1 1 1] Movement Input Binding
  (`TankMovementComponent.IntendTurnLeft` (`self.TankMovement`) AxisValue))

(event `InputAxis|MoveRight`
  (params (AxisValue :type "Float (single-precision)"))
  ;[1 1 1] Movement Input Binding
  (`TankMovementComponent.IntendTurnRight` (`self.TankMovement`) AxisValue))

(fn `UserConstructionScript`)